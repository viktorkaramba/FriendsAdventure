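; BP_Bucket is a Level 1 Stage 3 actor that receives fitting pieces carried by the player character.
; When a MyCharacter overlaps its Box holding a valid piece flagged Fit, it detaches that piece, moves it to the piece's own Point location and clears the character's reference.
; Each placement increments a Counter, which is only printed as debug output.
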(event OnComponentBeginOverlap(Box)
  (params (OverlappedComponent :type Primitive%20Component%20Object%20Reference) (OtherActor :type Actor%20Object%20Reference) (OtherComp :type Primitive%20Component%20Object%20Reference) (OtherBodyIndex :type Integer) (bFromSweep :type Boolean) (SweepResult :type Hit%20Result%20Structure%20%28by%20ref%29))
  (bind _asmy_character (Utilities|Casting|CastToMyCharacter OtherActor)
    (:then
      (Utilities|IsValid (Variables|/Game/MyCharacters/Main/MyCharacter.MyCharacter_C|GetCurrent_Piece _asmy_character)
        (:Is%20Valid
          (if (Variables|/Game/Levels/Level_1/Materials/Stage_3/BP_Piece_Base.BP_Piece_Base_C|Getfit (Variables|/Game/MyCharacters/Main/MyCharacter.MyCharacter_C|GetCurrent_Piece _asmy_character))
            (Transformation|DetachFromActor (Variables|/Game/MyCharacters/Main/MyCharacter.MyCharacter_C|GetCurrent_Piece _asmy_character) "KeepRelative" "KeepRelative" "KeepRelative")
            (Transformation|SetActorLocation (Variables|/Game/MyCharacters/Main/MyCharacter.MyCharacter_C|GetCurrent_Piece _asmy_character) (Variables|/Game/Levels/Level_1/Materials/Stage_3/BP_Piece_Base.BP_Piece_Base_C|GetPoint (Variables|/Game/MyCharacters/Main/MyCharacter.MyCharacter_C|GetCurrent_Piece _asmy_character)) false false)
            (Variables|/Game/MyCharacters/Main/MyCharacter.MyCharacter_C|SetCurrent_Piece _asmy_character 0)
            (bind _result (Math|Integer|IncrementInt (Variables|Default|GetCounter))
              (:%20%20
                (Development|PrintString (Utilities|String|ToString(Integer) _result))))))))
    (:CastFailed
      (Development|PrintString "No piece in character"))))

(fn ConstructionScript)